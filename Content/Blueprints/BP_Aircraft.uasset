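; Aircraft actor that flies along the spline of a referenced PlaneTrack.
; The MoveAirCraft event starts the AirCraftMover timeline at AircraftStartOffset, with play rate set to the inverse of Duration.
; Each timeline update maps Alpha to a distance along the spline and sets the actor's world transform, rotation included, without sweeping.
; Nothing in this Blueprint calls MoveAirCraft, and Tick is unused.
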(event `MoveAirCraft`
  (bind _aircraftmover (`self.AirCraftMover`))
  (`TimelineComponent.SetPlayRate` _aircraftmover (/ 1.0 (`self.Duration`)))
  (`TimelineComponent.SetNewTime` _aircraftmover (`self.AircraftStartOffset`))
  (bind (_direction _alpha) (`Timeline|AirCraftMover`)
    (:`Update`
      (set `self.Alpha` _alpha)
      (`self.K2_SetActorTransform` (`SplineComponent.GetTransformAtDistanceAlongSpline` (`PlaneTrack.SplineTrack` (`self.PlaneTrack`)) (`KismetMathLibrary.Lerp` 0.0 (`SplineComponent.GetSplineLength` (`PlaneTrack.SplineTrack` (`self.PlaneTrack`))) (`self.Alpha`)) "World" false)))))

(fn `UserConstructionScript`)